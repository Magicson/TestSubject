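; Player pawn for a side-scroller that acts as a travelling camera, gliding toward a focus camera actor set after an optional delay.
; Each tick it steps its location and camera offset toward that actor at the actor's travel speed, snapping when close.
; While travelling, the target character and its AI controller run in slow motion; on arrival normal time returns and the controller's Initialize is called every tick.
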(event `self.ReceiveBeginPlay`
  (bind _asbp_side_scroller_game_mode (cast `/Game/Blueprints/BP_SideScrollerGameMode` (`GameplayStatics.GetGameMode`)))
  (set `self.GameMode` _asbp_side_scroller_game_mode))

(event `self.ReceiveTick`
  (params (DeltaSeconds :type "Float (single-precision)"))
  (bind _charactertoactivate (`self.CharacterToActivate`))
  (bind _charactertoactivate_2 (`self.CharacterToActivate`))
  (bind _cameratofocus (`self.CameraToFocus`))
  (`/Engine/EditorBlueprintResources/StandardMacros.IsValid` _cameratofocus
    (:`Is Valid`
      (bind _cameralocation (`self.GetCameraActorLocation` _cameratofocus))
      (bind _returnvalue (`self.GetCameraRelativeLocation` _cameratofocus))
      (`self.K2_SetActorLocation` _cameralocation)
      (`SceneComponent.K2_SetRelativeLocation` (`self.Camera`) _returnvalue false false)
      (if (not (`self.IsTravelComplete`))
        (`/Engine/EditorBlueprintResources/StandardMacros.IsValid` (`self.CharacterToActivate`)
          (:`Is Valid`
            (bind _asai_controller (cast `/Game/Mannequin/AI/AI_Controller` (`self.GetController` _charactertoactivate)))
            (bind _output_get (set `Actor.CustomTimeDilation` 0.25 _asai_controller))
            (set `Actor.CustomTimeDilation` _output_get _charactertoactivate)))
        (else
          (`/Engine/EditorBlueprintResources/StandardMacros.IsValid` _charactertoactivate_2
            (:`Is Valid`
              (bind _asai_controller_2 (cast `/Game/Mannequin/AI/AI_Controller` (`self.GetController` _charactertoactivate_2)))
              (bind _output_get_2 (set `Actor.CustomTimeDilation` 1.0 _asai_controller_2))
              (set `Actor.CustomTimeDilation` _output_get_2 _charactertoactivate_2)
              (`/Game/Mannequin/AI/AI_Controller.Initialize` _asai_controller_2))))))))

(event `CameraAndCharacterToFocus`
  (params (Camera :type "/Game/Blueprints/CameraLocations Object Reference") (Character :type "/Game/SideScrollerBP/Blueprints/SideScrollerCharacter Object Reference") (Delay :type "Float (double-precision)"))
  (`KismetSystemLibrary.Delay` Delay)
  (`|ExecutionSequence`
    (:`then_0`
      (`/Engine/EditorBlueprintResources/StandardMacros.IsValid` Camera
        (:`Is Valid`
          (set `self.CameraToFocus` Camera))))
    (:`then_1`
      (`/Engine/EditorBlueprintResources/StandardMacros.IsValid` Character
        (:`Is Valid`
          (set `self.CharacterToActivate` Character))))))

(fn `GetCameraActorLocation`
  (params (CameraActor :type "/Game/Blueprints/CameraLocations Object Reference"))
  (returns (CameraLocation :type "Vector Structure"))
  (bind _returnvalue (`self.K2_GetActorLocation` CameraActor))
  (bind _returnvalue_2 (- (`self.K2_GetActorLocation`) _returnvalue))
  (if (> (`KismetMathLibrary.VSize` _returnvalue_2) 10.0)
    (set `self.IsTravelComplete` false)
    (return (- (`self.K2_GetActorLocation`) (* (`KismetMathLibrary.Normal` _returnvalue_2) (`/Game/Blueprints/CameraLocations.TravelSpeed` CameraActor))))
    (else
      (set `self.IsTravelComplete` true)
      (return _returnvalue))))

(fn `GetCameraRelativeLocation`
  (params (CameraActor :type "/Game/Blueprints/CameraLocations Object Reference"))
  (returns (ReturnValue :type "Vector Structure"))
  (bind _relativelocation (`SceneComponent.RelativeLocation` (`CameraActor.CameraComponent` CameraActor)))
  (bind _relativelocation_2 (`SceneComponent.RelativeLocation` (`self.Camera`)))
  (bind _returnvalue (- _relativelocation_2 _relativelocation))
  (if (> (`KismetMathLibrary.VSize` _returnvalue) 10.0)
    (return (- _relativelocation_2 (* (`KismetMathLibrary.Normal` _returnvalue) (`/Game/Blueprints/CameraLocations.TravelSpeed` CameraActor))))
    (else
      (return _relativelocation))))

(fn `UserConstructionScript`)
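; Contact trigger actor for a side-scroller that reports player contact to the game mode as a test subject interaction.
; It caches BP_SideScrollerGameMode on BeginPlay.
; When a SideScrollerCharacter begins overlapping its box while IsActive is set, it calls TestSubjectInteraction, passing its DeathCaused value as the interaction type along with its own up vector.
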(event `self.ReceiveBeginPlay`
  (bind _asbp_side_scroller_game_mode (cast `/Game/Blueprints/BP_SideScrollerGameMode` (`GameplayStatics.GetGameMode`)))
  (set `self.GameModeRef` _asbp_side_scroller_game_mode))

(event `self.Box.OnComponentBeginOverlap`
  (params (OverlappedComponent :type "PrimitiveComponent Object Reference") (OtherActor :type "Actor Object Reference") (OtherComp :type "PrimitiveComponent Object Reference") (OtherBodyIndex :type Integer) (bFromSweep :type Boolean) (SweepResult :type "HitResult Structure (by ref)"))
  (cast `/Game/SideScrollerBP/Blueprints/SideScrollerCharacter` OtherActor)
  (if (`self.IsActive?`)
    (`/Game/Blueprints/BP_SideScrollerGameMode.TestSubjectInteraction` :`self` (`self.GameModeRef`) :`TypeOfInteraction` (`self.DeathCaused`) :`OtherActorUpVector` (`self.GetActorUpVector`))))

(fn `UserConstructionScript`)
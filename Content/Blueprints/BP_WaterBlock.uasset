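; Side-scroller water block that reacts to Gravity and Temperature power changes by flipping its fall direction, freezing solid, heating or returning to water after a delay.
; Each state swaps Pawn and Visibility collision and sets the temperature material value that Tick animates, alongside mass-scaled gravity force.
; A character inside triggers GameMode interactions when frozen or hot, passing a grid-snapped transform for ice.
; Freezing box-traces for a specific contact hazard, disabling it and pinning the block.
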(event `self.ReceiveBeginPlay`
  (bind _returnvalue (`PrimitiveComponent.CreateDynamicMaterialInstance` (`self.StaticMeshComponent`) 0 "/Game/Materials/WaterMaterial.WaterMaterial"))
  (set `self.DynamicMaterial` _returnvalue)
  (bind _asbp_side_scroller_game_mode (cast `/Game/Blueprints/BP_SideScrollerGameMode` (`GameplayStatics.GetGameMode`)))
  (set `self.GameModeRef` _asbp_side_scroller_game_mode))

(event `/Game/Blueprints/BP_InteractInterface.ChangePower`
  (params (Power :type "/Game/Blueprints/BP_Powers Enum" :default "NewEnumerator0") (PowerState :type "/Game/Blueprints/BP_PowerStates Enum" :default "NewEnumerator0"))
  (switch `/Game/Blueprints/BP_Powers` Power
    (:`NewEnumerator0`
      (switch `/Game/Blueprints/BP_PowerStates` PowerState
        (:`NewEnumerator0`
          (set `self.GravityScalar` 2.0)
          (set `self.GravityScalarUnitary` 1.0))
        (:`NewEnumerator3`
          (set `self.GravityScalar` -2.0)
          (set `self.GravityScalarUnitary` -1.0))))
    (:`NewEnumerator1`
      (switch `/Game/Blueprints/BP_PowerStates` PowerState
        (:`NewEnumerator0`
          (`KismetSystemLibrary.Delay` (`/Game/Blueprints/BP_LevelInfo.TimeToUnfreezeUnheat` (`/Game/Blueprints/BP_SideScrollerGameMode.LevelInfo` (`self.GameModeRef`))))
          (`self.Unheat/Unfreze`))
        (:`NewEnumerator1`
          (`self.Heat`))
        (:`NewEnumerator2`
          (`self.Freze`))))))

(event `self.ReceiveTick`
  (params (DeltaSeconds :type "Float (single-precision)"))
  (bind _staticmeshcomponent (`self.StaticMeshComponent`))
  (if (not (`self.IsFixed`))
    (`PrimitiveComponent.AddForce` _staticmeshcomponent (* (* (0.0 0.0 -1000.0) (`PrimitiveComponent.GetMass` _staticmeshcomponent)) (`self.GravityScalar`)) "None" false))
  (`self.HandleMaterialAnimation`))

(event `self.Box.OnComponentBeginOverlap`
  (params (OverlappedComponent :type "PrimitiveComponent Object Reference") (OtherActor :type "Actor Object Reference") (OtherComp :type "PrimitiveComponent Object Reference") (OtherBodyIndex :type Integer) (bFromSweep :type Boolean) (SweepResult :type "HitResult Structure (by ref)"))
  (bind _asside_scroller_character (cast `/Game/SideScrollerBP/Blueprints/SideScrollerCharacter` OtherActor))
  (bind _output_get (set `self.InBoundsTestSubject` _asside_scroller_character))
  (bind _returnvalue (`self.GetTransform` _output_get))
  (set `self.SpawnTransform` (`KismetMathLibrary.MakeTransform` (`KismetMathLibrary.MakeVector` (.x (.location _returnvalue)) (`self.RoundTransform Y-Z` (.y (.location _returnvalue))) (`self.RoundTransform Y-Z` (.z (.location _returnvalue)))) (.rotation _returnvalue) (.scale _returnvalue)))
  (if (== (`self.MaterialToSetScalar`) -1.0)
    (`/Game/Blueprints/BP_SideScrollerGameMode.TestSubjectInteraction` :`self` (`self.GameModeRef`) :`TypeOfInteraction` "NewEnumerator3")))

(event `self.Box.OnComponentEndOverlap`
  (params (OverlappedComponent :type "PrimitiveComponent Object Reference") (OtherActor :type "Actor Object Reference") (OtherComp :type "PrimitiveComponent Object Reference") (OtherBodyIndex :type Integer))
  (cast `/Game/SideScrollerBP/Blueprints/SideScrollerCharacter` OtherActor)
  (set `self.InBoundsTestSubject` null))

(fn `Freze`
  (bind _returnvalue (`self.K2_GetActorLocation`))
  (set `self.MaterialToSetScalar` 1.0)
  (`PrimitiveComponent.SetCollisionResponseToChannel` (`self.StaticMeshComponent`) "ECC_Visibility" "ECR_Block")
  (`PrimitiveComponent.SetCollisionResponseToChannel` (`self.StaticMeshComponent`) "ECC_Pawn" "ECR_Block")
  (set `self.IsFrozen` true)
  (bind _outhit (`KismetSystemLibrary.BoxTraceSingle` _returnvalue _returnvalue (30.0 30.0 30.0) (struct) "TraceTypeQuery1"))
  (`self.Fix/Unfix` (`.HitActor` (`GameplayStatics.BreakHitResult` _outhit)) true)
  (`/Engine/EditorBlueprintResources/StandardMacros.IsValid` (`self.InBoundsTestSubject`)
    (:`Is Valid`
      (set `self.InBoundsTestSubject` null)
      (`/Game/Blueprints/BP_SideScrollerGameMode.TestSubjectInteraction` (`self.GameModeRef`) "NewEnumerator2" (0.0 0.0 0.0) (`self.SpawnTransform`)))))

(fn `HandleMaterialAnimation`
  (bind _currentmaterialscalar (`self.CurrentMaterialScalar`))
  (if (> (`self.MaterialToSetScalar`) _currentmaterialscalar)
    (bind _output_get (set `self.CurrentMaterialScalar` (`KismetMathLibrary.FClamp` (+ _currentmaterialscalar 0.05) -1.0)))
    (else
      (set `self.CurrentMaterialScalar` (`KismetMathLibrary.FClamp` (- _currentmaterialscalar 0.05) -1.0))))
  (`MaterialInstanceDynamic.SetScalarParameterValue` (`self.DynamicMaterial`) "Temperature Level" _output_get))

(fn `Heat`
  (set `self.MaterialToSetScalar` -1.0)
  (`PrimitiveComponent.SetCollisionResponseToChannel` (`self.StaticMeshComponent`) "ECC_Visibility" "ECR_Ignore")
  (`PrimitiveComponent.SetCollisionResponseToChannel` (`self.StaticMeshComponent`) "ECC_Pawn" "ECR_Overlap")
  (set `self.IsFrozen` false)
  (set `self.IsFixed` false)
  (`/Engine/EditorBlueprintResources/StandardMacros.IsValid` (`self.InBoundsTestSubject`)
    (:`Is Valid`
      (set `self.InBoundsTestSubject` null)
      (`/Game/Blueprints/BP_SideScrollerGameMode.TestSubjectInteraction` :`self` (`self.GameModeRef`) :`TypeOfInteraction` "NewEnumerator3"))))

(fn `IsFrozen?`
  (returns (`IsFrozen?` :type Boolean))
  (return (`self.IsFrozen`)))

(fn `RoundTransform Y-Z`
  (params (Coordinate :type "Float (double-precision)"))
  (returns (`Rounded Coordinate` :type "Float (double-precision)"))
  (bind (_remainder _returnvalue) (`KismetMathLibrary.FMod` Coordinate 100.0))
  (bind _returnvalue_2 (* _returnvalue 100))
  (if (> _remainder 49.0)
    (return (`KismetMathLibrary.Conv_IntToDouble` (+ _returnvalue_2 100)))
    (else
      (return (`KismetMathLibrary.Conv_IntToDouble` _returnvalue_2)))))

(fn `Unheat/Unfreze`
  (bind _returnvalue (`self.K2_GetActorLocation`))
  (bind _bp_powerstruct (`/Game/Blueprints/BP_SideScrollerGameMode.GetPowerState` (`self.GameModeRef`) "NewEnumerator1"))
  (switch `/Game/Blueprints/BP_PowerStates` _bp_powerstruct
    (:`NewEnumerator0`
      (set `self.MaterialToSetScalar` 0.0)
      (`PrimitiveComponent.SetCollisionResponseToChannel` (`self.StaticMeshComponent`) "ECC_Visibility" "ECR_Ignore")
      (`PrimitiveComponent.SetCollisionResponseToChannel` (`self.StaticMeshComponent`) "ECC_Pawn" "ECR_Overlap")
      (set `self.IsFrozen` false)
      (bind _outhit (`KismetSystemLibrary.BoxTraceSingle` _returnvalue _returnvalue (30.0 30.0 30.0) (struct) "TraceTypeQuery1"))
      (`self.Fix/Unfix` (`.HitActor` (`GameplayStatics.BreakHitResult` _outhit))))))

(fn `UserConstructionScript`)
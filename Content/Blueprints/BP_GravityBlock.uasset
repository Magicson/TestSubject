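; BP_GravityBlock is a physics block whose gravity can be flipped by a power change.
; The ChangePower event sets a gravity scalar to a positive or negative value for the Normal or Inverted state of the Gravity power.
; Each Tick, it applies a mass-scaled vertical force to its static mesh, multiplied by that scalar, pushing the block down or up.
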(event `/Game/Blueprints/BP_InteractInterface.ChangePower`
  (params (Power :type "/Game/Blueprints/BP_Powers Enum") (PowerState :type "/Game/Blueprints/BP_PowerStates Enum"))
  (switch `/Game/Blueprints/BP_Powers` Power
    (:`NewEnumerator0`
      (switch `/Game/Blueprints/BP_PowerStates` PowerState
        (:`NewEnumerator0`
          (set `self.GravityScalar` 2.0))
        (:`NewEnumerator3`
          (set `self.GravityScalar` -2.0))))))

(event `self.ReceiveTick`
  (params (DeltaSeconds :type "Float (single-precision)"))
  (bind _staticmeshcomponent (`self.StaticMeshComponent`))
  (`PrimitiveComponent.AddForce` _staticmeshcomponent (* (* (0.0 0.0 -1000.0) (`PrimitiveComponent.GetMass` _staticmeshcomponent)) (`self.GravityScalar`)) "None" false))

(fn `UserConstructionScript`)